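; BP_Car is a car actor for the Crossy Road game that drives continuously along its local Y axis.
; BeginPlay picks a random move speed, keeps a copy in Matchspeed and spawns an attached car sound.
; Tick applies that speed as a per-frame local offset without delta-time scaling.
; The overlap event is empty, and a disconnected branch for speed matching or a swept sideways shift never runs.
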(event EventBeginPlay
  (Variables|Default|SetMoveSpeed (Math|Random|RandomFloatinRange 1.0 6.0))
  (Variables|Default|SetMatchspeed (Variables|Default|GetMoveSpeed))
  (Audio|SpawnSoundAttached "/Game/CrossyRoad/Sounds/cari.cari" 0 "None" "0, 0, 0" "0, 0, 0" "KeepRelativeOffset" false 1.0 1.0 0.0 0 0))

(event EventTick
  (params (DeltaSeconds :type Float%20%28single-precision%29))
  (Transformation|AddActorLocalOffset (Math|Vector|MakeVector 0.0 (Variables|Default|GetMoveSpeed) 0.0) false false))

(event Collision|EventActorBeginOverlap
  (params (OtherActor :type Actor%20Object%20Reference)))

(fn ConstructionScript)